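; Door actor that swings open and closed in response to DoorEvent open and close events.
; It caches its starting rotation on BeginPlay, and the TL_DoorSwing timeline adds an animated yaw angle to it, so the swing is relative to the door's placed orientation.
; Opening plays the timeline, closing reverses it, and a timeline event track plays a sound at the door's location.
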(event `self.ReceiveBeginPlay`
  (set `self.InitRotation` (`self.K2_GetActorRotation`)))

(event `self.DoorEvent.OnOpen`
  (bind (_direction _open_angle) (`Timeline|TL_DoorSwing` :!label _label)
    (:`Update`
      (`self.K2_SetActorRotation` (`KismetMathLibrary.ComposeRotators` (`KismetMathLibrary.MakeRotator` 0.0 0.0 _open_angle) (`self.InitRotation`))))
    (:`SoundTiming`
      (`GameplayStatics.PlaySoundAtLocation` "/Game/StarterContent/Audio/Collapse01.Collapse01" (`self.K2_GetActorLocation`) (struct) 0.5))))

(event `self.DoorEvent.OnClose`
  (goto _label :!via `Reverse`))

(fn `UserConstructionScript`)